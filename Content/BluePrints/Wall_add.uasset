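; Wall_add is a Blueprint for a wall that displays an additive value as a "+" label.
; On BeginPlay it formats TextValue with a plus prefix and writes it to TextObject.
; The SpawnCollision overlap event is empty, with disconnected branch, interface-check and destroy nodes left in the graph.
; TriggerIncreaseSpawn and IncreaseSpawnQuantity are stubs returning zero, so the wall does not change any spawn count itself.
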(event `self.SpawnCollision.OnComponentBeginOverlap`
  (params (OverlappedComponent :type "PrimitiveComponent Object Reference") (OtherActor :type "Actor Object Reference") (OtherComp :type "PrimitiveComponent Object Reference") (OtherBodyIndex :type Integer) (bFromSweep :type Boolean) (SweepResult :type "HitResult Structure (by ref)")))

(event `self.ReceiveBeginPlay`
  (`TextRenderComponent.K2_SetText` (`self.TextObject`) (`KismetTextLibrary.Conv_StringToText` (`KismetStringLibrary.Concat_StrStr` "+ " (`KismetTextLibrary.Conv_TextToString` (`KismetTextLibrary.Conv_IntToText` (`self.textValue`)))))))

(fn `IncreaseSpawnQuantity`
  (params (input :type Integer :default 0))
  (returns (result :type Integer))
  (return 0))

(fn `TriggerIncreaseSpawn`
  (params (Input :type Integer :default 0))
  (returns (Output :type Integer))
  (return 0))

(fn `UserConstructionScript`)